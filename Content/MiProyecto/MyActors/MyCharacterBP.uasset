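; Player character Blueprint that tracks firing state and plays visual effects for shooting and jumping.
; Fire2 input and shoot start/stop events set IsFire, with the latter also toggling a particle component.
; Jumps and ShootSceneComponent hits spawn emitters at the actor and hit point.
; An unconnected camera multi-trace would reduce damage through ParedBP walls and subtract it from EnemyBP health; helper functions are empty.
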(event `InputAction|Fire2` :overrideparent false
  (params (Key :type "Key Structure"))
  (:`Pressed`
    (set `self.isFire` true))
  (:`Released`
    (set `self.isFire` false)))

(event `self.OnStartShoot`
  (set `self.isFire` true)
  (`ActorComponent.Activate` (`self.ParticleSystem`) false))

(event `self.OnStopShoot`
  (set `self.isFire` false)
  (`ActorComponent.Deactivate` (`self.ParticleSystem`)))

(event `self.OnStartJump`
  (bind (_returnvalue_location _returnvalue_rotation _returnvalue_scale) (`KismetMathLibrary.BreakTransform` (`self.GetTransform`)))
  (`GameplayStatics.SpawnEmitterAtLocation` "/Game/MiProyecto/Particle/ParticleSystem.ParticleSystem" _returnvalue_location _returnvalue_rotation _returnvalue_scale))

(event `self.shootSceneComponent.onHit`
  (params (hitPoint :type "Vector Structure"))
  (`GameplayStatics.SpawnEmitterAtLocation` "/Game/MiProyecto/Particle/ParticleSystem.ParticleSystem" hitPoint))

(fn `NewFunction_0`
  (params (TargetArray :type "Array of HitResult Structure (by ref)")))

(fn `NewFunction_1`
  (params (TargetArray :type "Array of HitResult Structure (by ref)")))

(fn `UserConstructionScript`)