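; Behavior Tree task that picks the next patrol waypoint for an AI-controlled PatrolBP pawn.
; On execute it reads the pawn's waypoints, advances the current index, wraps to the first after the last, and reports success.
; The NuevaPos helper writes that waypoint actor's location to a Blackboard vector key.
; Other pawn types fail the task with a debug message; unconnected random-position and alternate-increment logic remains unused.
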(event `self.ReceiveExecuteAI`
  (params (OwnerController :type "AIController Object Reference") (ControlledPawn :type "Pawn Object Reference"))
  (bind _aspatrol_bp (cast `/Game/MiProyecto/PatrolBP` ControlledPawn)
    (:`then`
      (bind _targetpoints (`/Game/MiProyecto/PatrolBP.GetWayPoints` _aspatrol_bp))
      (set `self.TargetPoints` _targetpoints)
      (if (< (`self.CurrentWayPoint`) (- (`KismetArrayLibrary.Array_Length` (`self.TargetPoints`)) 1))
        (set `self.CurrentWayPoint` (+ 1 (`self.CurrentWayPoint`)))
        (`self.NuevaPos`)
        (`self.FinishExecute` true)
        (else
          (set `self.CurrentWayPoint` 0)
          (`self.NuevaPos`)
          (`self.FinishExecute` true))))
    (:`CastFailed`
      (`self.FinishExecute` false)
      (`KismetSystemLibrary.PrintString` "El objeto no es patrullable"))))

(fn `NuevaPos`
  (`BTFunctionLibrary.SetBlackboardValueAsVector` (`self.StructValues`) (`Actor.K2_GetActorLocation` (`|GetArrayItem` (`self.TargetPoints`) (`self.CurrentWayPoint`)))))